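; Side-scrolling sprite player character, a bunny that transforms through Ball, Front Legs, Ears and Back Legs states, unlocking jump, brake, glide and double jump.
; InitMoveState sets friction, anim instance, VFX and thought-bubble key prompts per state.
; Tick locks Y, flips the sprite and traces for ground, while timelines drive glide gravity and braking.
; It also takes wind launches scaled by braking, tracks three collectibles in a widget, and has debug state cycling.
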(event Custom|Update%20Player%20Rotation
  (bind _sprite (Variables|Default|GetSprite))
  ;[0.15 0.15 0.15 0.5] Flip character based on which way they are moving
  (switch Utilities|FlowControl|Switch|SwitchonE_PlayerMoveState (Variables|Default|GetPlayerMovementState)
    (:NewEnumerator0
      _)
    (:NewEnumerator1
      _)
    (:NewEnumerator2
      _)
    (:NewEnumerator3
      _))
  (Math|Float|CompareFloat (Variables|Default|GetInput%20Direction) 0.0
    (:>
      (Transformation|SetRelativeRotation _sprite "0, 0, 0" false false))
    (:<
      (Transformation|SetRelativeRotation _sprite "0.000000,180.000000,0.000000" false false))))

(event Custom|BlowCharacter
  (params (BlowVelocity :type Float%20%28double-precision%29))
  ;[0.15 0.15 0.15 0.5] Blow tick
  (if (Variables|Default|GetIsBreaking)
    (Character|LaunchCharacter (Math|Vector|MakeVector (* BlowVelocity (Variables|Default|GetBlow%20Strength%20Breaking)) 0.0 0.0) false false)
    (else
      (Character|LaunchCharacter (Math|Vector|MakeVector (* BlowVelocity (Variables|Default|GetBlow%20Strength%20Normal)) 0.0 0.0) false false))))

(event Custom|CheckEndBlow
  ;[0.15 0.15 0.15 0.5] Blow End
  (if (and (Variables|Default|GetIsBlown) (!= (Variables|/Game/Blueprints/Environment/BP_EnvironmentManager.BP_EnvironmentManager_C|GetIsEnvironmentEffectActive (Variables|Default|GetEnvironment%20Manager)) true))
    (Utilities|FlowControl|Delay 0.2)
    (Variables|Default|SetIsBlown (>= (Math|Float|Absolute(Float) (Math|Vector|VectorLengthXY (Transformation|GetVelocity))) (Variables|/Game/Blueprints/AnimationBlueprints/BP_AnimBallState.BP_AnimBallState_C|GetIdle%20Anim%20Velocity (Variables|Default|GetPlayer%20Animation))))
    (CallFunction|InitMoveState)))

(event Custom|Init%20Vars
  ;[0.15 0.15 0.15 0.5] Init vars (storing object references on start so more efficient)
  (bind _asbp_anim_ball_state (Utilities|Casting|CastToBP_AnimBallState (Variables|/Script/PaperZD.PaperZDAnimationComponent|GetAnimInstance (Variables|Default|GetAnimationComponent))))
  (Variables|Default|SetPlayer%20Animation _asbp_anim_ball_state)
  (bind _returnvalue (Actor|GetActorOfClass "/Game/Blueprints/Environment/BP_EnvironmentManager.BP_EnvironmentManager_C"))
  (Variables|Default|SetEnvironment%20Manager _returnvalue)
  (Variables|Default|SetStarting%20Y%20Pos (.y (.location (Transformation|GetActorTransform))))
  (bind _returnvalue_2 (UserInterface|CreateWidget "/Game/UI/WBP_CollectedIteams.WBP_CollectedIteams_C"))
  (UserInterface|Viewport|AddtoPlayerScreen _returnvalue_2)
  (Variables|Default|SetCollectionWidgetReference _returnvalue_2))

(event Custom|Check%20Y%20Position
  (bind _returnvalue (Transformation|GetActorLocation))
  (bind _starting_y_pos (Variables|Default|GetStarting%20Y%20Pos))
  ;[0.15 0.15 0.15 0.5] Lock character position on Y axis
  (if (!= (.y _returnvalue) _starting_y_pos)
    (Transformation|SetActorLocation (Math|Vector|MakeVector (.x _returnvalue) _starting_y_pos (.z _returnvalue)) false false)))

(event Custom|Update%20Debug%20Text
  ;[0.15 0.15 0.15 0.5] Print current speed ratio and current movement type
  (Rendering|Components|TextRender|SetText (Variables|Default|GetDebugStateText) (Utilities|Text|FormatText "{movement} {velocity} " (|GenerictoText (Variables|Default|GetPlayerMovementState)) (/ (.x (Transformation|GetVelocity)) (Variables|/Script/Engine.CharacterMovementComponent|GetMaxWalkSpeed (Variables|Character|GetCharacterMovement))))))

(event Custom|Init%20Blow
  (bind _charactermovement (Variables|Character|GetCharacterMovement))
  ;[0.15 0.15 0.15 0.5] Blow Init
  (Variables|Default|SetIsBlown true)
  ;;[0.15 0.15 0.15 0.5] Set ball friction and accelleration to 0 when wind is winding
  (if (== (Variables|Default|GetPlayerMovementState) 0)
    (Variables|/Script/Engine.CharacterMovementComponent|SetMaxAcceleration _charactermovement 0.0)
    (Variables|/Script/Engine.CharacterMovementComponent|SetGroundFriction _charactermovement 0.0)))

(event Custom|CheckGrounded
  (bind _helicopter (Variables|Default|GetHelicopter))
  (bind _capsulecomponent (Variables|Collision|GetCapsuleComponent))
  (bind _returnvalue (Transformation|GetWorldLocation _capsulecomponent))
  (bind _capsulehalfheight (Variables|/Script/Engine.CapsuleComponent|GetCapsuleHalfHeight _capsulecomponent))
  (bind _returnvalue_2 (- _returnvalue (Math|Vector|MakeVector 0.0 0.0 _capsulehalfheight)))
  ;[0.15 0.15 0.15 0.5] grounded check
  (bind _returnvalue_3 (Collision|LineTraceForObjects _returnvalue_2 (+ _returnvalue_2 "0.000000,0.000000,-10.000000") (Utilities|Array|MakeArray "ObjectTypeQuery1") false 0 "None"))
  (bind _output_get (Variables|Default|SetIsGrounded _returnvalue_3))
  (Variables|/Script/Engine.CharacterMovementComponent|SetGravityScale (Variables|Character|GetCharacterMovement) 1.0)
  (if _output_get
    (Variables|Default|SetIsDoubleJumping false)
    (if (Utilities|IsValid _helicopter)
      (Audio|Components|Audio|FadeOut _helicopter 0.0 0.0 "Linear" :!class /Script/Engine.AudioComponent))))

(event Custom|ProcessGlide
  (bind _charactermovement (Variables|Character|GetCharacterMovement))
  (bind _helicopter (Variables|Default|GetHelicopter))
  ;[0.15 0.15 0.15 0.5] jumping  (and gliding)
  ;;[0.15 0.15 0.15 0.5] Glide
  (if (Variables|Default|GetIsGliding)
    (bind _glidetime (Timeline|Glide Play)
      (:Update
        (Variables|/Script/Engine.CharacterMovementComponent|SetGravityScale _charactermovement _glidetime))
      (:Finished
        (Variables|/Script/Engine.CharacterMovementComponent|SetGravityScale _charactermovement 1.0)))
    (elif (Utilities|IsValid _helicopter)
      (Audio|Components|Audio|FadeOut _helicopter 0.2 0.0 "Linear" :!class /Script/Engine.AudioComponent)
      (Timeline|Glide Stop)
      (else
        (Timeline|Glide Stop)))))

(event Custom|CloseAfterTime
  (Timeline|ShowPromptTime PlayFromStart
    (:Finished
      (CallFunction|HideBubble))))

(event Input|EnhancedActionEvents|EnhancedInputActionIA_Running
  (params (ActionValue :type Float%20%28double-precision%29) (ElapsedSeconds :type Float%20%28double-precision%29) (TriggeredSeconds :type Float%20%28double-precision%29) (InputAction :type Input%20Action%20Object%20Reference :default "/Game/Blueprints/IA_Running.IA_Running"))
  ;[0.15 0.15 0.15 0.5] Horizontal Movement Input
  (:Triggered
    (bind _output_get (Variables|Default|SetInput%20Direction ActionValue))
    (if (not (Variables|Default|GetIsBreaking))
      (Pawn|Input|AddMovementInput "1.000000,0.000000,0.000000" _output_get false)
      (Variables|Default|SetIsHorzMovement true)))
  (:Completed
    (Variables|Default|SetIsHorzMovement false)))

(event Input|EnhancedActionEvents|EnhancedInputActionIA_StateChange
  (params (ActionValue :type Boolean) (ElapsedSeconds :type Float%20%28double-precision%29) (TriggeredSeconds :type Float%20%28double-precision%29) (InputAction :type Input%20Action%20Object%20Reference :default "/Game/Blueprints/IA_StateChange.IA_StateChange"))
  ;[0.15 0.15 0.15 0.5] Debug State Change
  (switch Utilities|FlowControl|Switch|SwitchonE_PlayerMoveState (Variables|Default|GetPlayerMovementState)
    (:NewEnumerator0
      (CallFunction|ChangeMovementState "NewEnumerator1"))
    (:NewEnumerator1
      (CallFunction|ChangeMovementState "NewEnumerator2"))
    (:NewEnumerator2
      (CallFunction|ChangeMovementState "NewEnumerator3"))
    (:NewEnumerator3
      (CallFunction|ChangeMovementState "NewEnumerator0"))))

(event Input|EnhancedActionEvents|EnhancedInputActionIA_Jumping
  (params (ActionValue :type Boolean) (ElapsedSeconds :type Float%20%28double-precision%29) (TriggeredSeconds :type Float%20%28double-precision%29) (InputAction :type Input%20Action%20Object%20Reference :default "/Game/Blueprints/IA_Jumping.IA_Jumping"))
  (bind _charactermovement (Variables|Character|GetCharacterMovement))
  ;[0.15 0.15 0.15 0.5] jumping  (and gliding)
  (:Started
    ;;[0.15 0.15 0.15 0.5] First Jump
    (if (and (and (not (Variables|Default|GetIsJumping)) (Variables|Default|GetIsGrounded)) (> (Variables|Default|GetPlayerMovementState) 0))
      (Variables|Default|SetIsJumping true)
      (if (== (Variables|Default|GetPlayerMovementState) 3)
        (Character|LaunchCharacter (Math|Vector|MakeVector 0.0 0.0 (Variables|Default|GetJump%20Velocity%20Big)) false false)
        (else
          (Character|LaunchCharacter (Math|Vector|MakeVector 0.0 0.0 (Variables|Default|GetJump%20Velocity%20Normal)) false false)))
      (else
        ;;[0.15 0.15 0.15 0.5] Double Jump
        (if (Math|Boolean|ANDBoolean (not (Variables|Default|GetIsGrounded)) (== (Variables|Default|GetPlayerMovementState) 3) (not (Variables|Default|GetIsDoubleJumping)))
          (Variables|Default|SetIsDoubleJumping true)
          (Character|LaunchCharacter (Math|Vector|MakeVector 0.0 0.0 (Variables|Default|GetJump%20Velocity%20Double)) false false))
        ;;[0.15 0.15 0.15 0.5] Glide
        (if (and (not (Variables|Default|GetIsGrounded)) (or (== (Variables|Default|GetPlayerMovementState) 2) (and (== (Variables|Default|GetPlayerMovementState) 3) (Variables|Default|GetIsDoubleJumping))))
          (Variables|Default|SetIsGliding true)
          (bind _returnvalue (Audio|SpawnSound2D "/Game/Audio/SoundEffects/Helicopter2.Helicopter2" 0.4 0.85 0.0 0))
          (Audio|Components|Audio|FadeIn _returnvalue 0.1 1.0 0.0 "Linear" :!class /Script/Engine.AudioComponent)
          (Variables|Default|SetHelicopter _returnvalue)
          (bind _glidetime (Timeline|Glide PlayFromStart)
            (:Update
              (Variables|/Script/Engine.CharacterMovementComponent|SetGravityScale _charactermovement _glidetime))
            (:Finished
              (Variables|/Script/Engine.CharacterMovementComponent|SetGravityScale _charactermovement 1.0)))))))
  (:Canceled
    ;;[0.15 0.15 0.15 0.5] reset jump/glide states
    (Variables|Default|SetIsJumping false :!label _label)
    (Variables|Default|SetIsGliding false)
    (Variables|/Script/Engine.CharacterMovementComponent|SetGravityScale (Variables|Character|GetCharacterMovement) 1.0))
  (:Completed
    (goto _label)))

(event Input|EnhancedActionEvents|EnhancedInputActionIA_Braking
  (params (ActionValue :type Boolean) (ElapsedSeconds :type Float%20%28double-precision%29) (TriggeredSeconds :type Float%20%28double-precision%29) (InputAction :type Input%20Action%20Object%20Reference :default "/Game/Blueprints/IA_Braking.IA_Braking"))
  (bind _charactermovement (Variables|Character|GetCharacterMovement))
  ;[0.15 0.15 0.15 0.5] Bunny breaks (once front legs are obtained)
  (:Triggered
    (if (and (!= (Variables|Default|GetPlayerMovementState) 0) (Variables|Default|GetIsGrounded)) :!label _label
      (bind _velocity_reduction_ratio (Timeline|Break%20Timeline Play)
        (:Update
          (Variables|/Script/Engine.MovementComponent|SetVelocity _charactermovement (Math|Vector|MakeVector (* _velocity_reduction_ratio (.x (Variables|/Script/Engine.MovementComponent|GetVelocity _charactermovement))) 0.0 (.z (Variables|/Script/Engine.MovementComponent|GetVelocity _charactermovement))))
          (Variables|Default|SetIsBreaking true)
          (if (Variables|Default|GetIsJumping)
            (Timeline|Break%20Timeline Stop)
            (elif (<= (Math|Float|Absolute(Float) (.x (Variables|/Script/Engine.MovementComponent|GetVelocity _charactermovement))) 5e+01)
              (Timeline|Break%20Timeline Stop)
              (elif (not (Variables|Default|GetIsGrounded))
                (Timeline|Break%20Timeline Stop)
                (else
                  (Timeline|Break%20Timeline Play))))))
        (:Finished
          (Variables|/Script/Engine.MovementComponent|SetVelocity _charactermovement (Math|Vector|MakeVector (* (.x (Variables|/Script/Engine.MovementComponent|GetVelocity _charactermovement)) 0.01) 0.0 (.z (Variables|/Script/Engine.MovementComponent|GetVelocity _charactermovement))))))
      (else
        (Timeline|Break%20Timeline Stop))))
  (:Started
    (if (and (and (!= (Variables|Default|GetPlayerMovementState) 0) (not (Variables|Default|GetIsJumping))) (Variables|Default|GetIsGrounded))
      (Timeline|Break%20Timeline PlayFromStart)
      (else
        (Timeline|Break%20Timeline Stop))))
  (:Ongoing
    (goto _label))
  (:Canceled
    (Variables|Default|SetIsBreaking false :!label _label_2)
    (Timeline|Break%20Timeline Stop))
  (:Completed
    (goto _label_2)))

(event EventBeginPlay
  (bind _returnvalue (Game|GetPlayerController 0))
  (bind _returnvalue_2 (PlayerController|LocalPlayerSubsystems|GetEnhancedInputLocalPlayerSubsystem _returnvalue))
  (CallFunction|InitVars)
  (CallFunction|InitMoveState)
  (Utilities|IsValid _returnvalue_2
    (:Is%20Valid
      (Input|AddMappingContext _returnvalue_2 "/Game/Blueprints/IMC_PlayerMappingContext.IMC_PlayerMappingContext" 0 "(bIgnoreAllPressedKeysUntilRelease=True,bForceImmediately=False,bNotifyUserSettings=False)")
      (Utilities|FlowControl|Delay 4.0)
      (Rendering|SetVisibility (Variables|Default|GetThoughtBubble) true false)
      (Utilities|FlowControl|Delay 1e+01)
      (CallFunction|HideBubble))))

(event EventTick
  (params (DeltaSeconds :type Float%20%28single-precision%29))
  (CallFunction|CheckYPosition)
  (CallFunction|UpdatePlayerRotation)
  (CallFunction|CheckEndBlow)
  (CallFunction|UpdateDebugText)
  (CallFunction|CheckGrounded)
  (CallFunction|ProcessGlide))

(event Input|KeyboardEvents|E
  (params (Key :type Key%20Structure :default "None"))
  ;[0.15 0.15 0.15 0.5] Bunny breaks (once front legs are obtained)
  (:Pressed
    (Default|DebugEnviroTrigger (Variables|Default|GetEnvironment%20Manager))))

(fn ConstructionScript)

(fn ChangeMovementState
  (params (PlayerMovementState :type E_PlayerMoveState%20Enum :default "NewEnumerator0"))
  (Variables|Default|SetPlayerMovementState PlayerMovementState)
  (Audio|PlaySound2D "/Game/Audio/SoundEffects/sparkle.sparkle" 0.2 0.8 0.3 0 0 false)
  (CallFunction|InitMoveState))

(fn SetCollectedItems
  (params (ItemType :type BP%20Item%20Parent%20Class%20Reference))
  ;[0.15 0.15 0.15 0.5] Update which items have been collected
  (if (and (== ItemType "/Game/Blueprints/NPCs/Items/ItemsWantedByNPCs/BP_Item1.BP_Item1_C") (not (Variables|CollectedItems|GetHasItem1?)))
    (Variables|CollectedItems|SetHasItem1? true)
    (Default|ShowCollectedIcons (Variables|Default|GetCollectionWidgetReference) "Item1")
    (Audio|PlaySound2D "/Game/Audio/SoundEffects/Item_Grab.Item_Grab" 0.2 0.9 0.05 0 0 false :!label _label)
    (Audio|PlaySound2D "/Game/Audio/SoundEffects/sparkle_2.sparkle_2" 2.0 1.0 0.05 0 0 false)
    (return)
    (elif (and (== ItemType "/Game/Blueprints/NPCs/Items/ItemsWantedByNPCs/BP_Item2.BP_Item2_C") (not (Variables|CollectedItems|GetHasItem2?)))
      (Variables|CollectedItems|SetHasItem2? true)
      (Default|ShowCollectedIcons (Variables|Default|GetCollectionWidgetReference) "Item2")
      (goto _label)
      (elif (and (== ItemType "/Game/Blueprints/NPCs/Items/ItemsWantedByNPCs/BP_Item3.BP_Item3_C") (not (Variables|CollectedItems|GetHasItem3?)))
        (Variables|CollectedItems|SetHasItem3? true)
        (Default|ShowCollectedIcons (Variables|Default|GetCollectionWidgetReference) "Item3")
        (goto _label)))))

(fn GetCollectedItems
  (params (ItemToCheck :type BP%20Item%20Parent%20Class%20Reference))
  ;[0.15 0.15 0.15 0.5] Return which item has been collected
  (if (and (== ItemToCheck "/Game/Blueprints/NPCs/Items/ItemsWantedByNPCs/BP_Item1.BP_Item1_C") (Variables|CollectedItems|GetHasItem1?))
    (return true)
    (elif (and (== ItemToCheck "/Game/Blueprints/NPCs/Items/ItemsWantedByNPCs/BP_Item2.BP_Item2_C") (Variables|CollectedItems|GetHasItem2?))
      (return true)
      (elif (and (== ItemToCheck "/Game/Blueprints/NPCs/Items/ItemsWantedByNPCs/BP_Item3.BP_Item3_C") (Variables|CollectedItems|GetHasItem3?))
        (return true)
        (else
          (return false))))))

(fn InitMoveState
  (bind _charactermovement (Variables|Character|GetCharacterMovement))
  (bind _charactermovement_2 (Variables|Character|GetCharacterMovement))
  (bind _charactermovement_3 (Variables|Character|GetCharacterMovement))
  (bind _charactermovement_4 (Variables|Character|GetCharacterMovement))
  (bind _sprite (Variables|Default|GetSprite))
  (bind _origin (Collision|GetComponentBounds _sprite))
  (bind _returnvalue (+ (.y _origin) 1e+01))
  (switch Utilities|FlowControl|Switch|SwitchonE_PlayerMoveState (Variables|Default|GetPlayerMovementState)
    (:NewEnumerator0
      (Variables|/Script/Engine.CharacterMovementComponent|SetMaxAcceleration _charactermovement 4e+02)
      (Variables|/Script/Engine.CharacterMovementComponent|SetGroundFriction _charactermovement 1.0)
      (Variables|/Script/Engine.CharacterMovementComponent|SetBrakingDecelerationWalking _charactermovement 0.5)
      (Class|PaperZDAnimationComponent|SetAnimInstanceClass (Variables|Default|GetAnimationComponent) "/Game/Blueprints/AnimationBlueprints/BP_AnimBallState.BP_AnimBallState_C"))
    (:NewEnumerator1
      (Variables|/Script/Engine.CharacterMovementComponent|SetMaxAcceleration _charactermovement_4 4e+02)
      (Variables|/Script/Engine.CharacterMovementComponent|SetGroundFriction _charactermovement_4 1.5)
      (Variables|/Script/Engine.CharacterMovementComponent|SetBrakingDecelerationWalking _charactermovement_4 1.0)
      (Class|PaperZDAnimationComponent|SetAnimInstanceClass (Variables|Default|GetAnimationComponent) "/Game/Blueprints/AnimationBlueprints/BP_AnimFrontLegsState.BP_AnimFrontLegsState_C"))
    (:NewEnumerator2
      (Variables|/Script/Engine.CharacterMovementComponent|SetMaxAcceleration _charactermovement_3 4e+02)
      (Variables|/Script/Engine.CharacterMovementComponent|SetGroundFriction _charactermovement_3 1.5)
      (Variables|/Script/Engine.CharacterMovementComponent|SetBrakingDecelerationWalking _charactermovement_3 1.0)
      (Class|PaperZDAnimationComponent|SetAnimInstanceClass (Variables|Default|GetAnimationComponent) "/Game/Blueprints/AnimationBlueprints/BP_AnimEarsState.BP_AnimEarsState_C"))
    (:NewEnumerator3
      (Variables|/Script/Engine.CharacterMovementComponent|SetMaxAcceleration _charactermovement_2 4e+02)
      (Variables|/Script/Engine.CharacterMovementComponent|SetGroundFriction _charactermovement_2 2.5)
      (Variables|/Script/Engine.CharacterMovementComponent|SetBrakingDecelerationWalking _charactermovement_2 3.0)
      (Class|PaperZDAnimationComponent|SetAnimInstanceClass (Variables|Default|GetAnimationComponent) "/Game/Blueprints/AnimationBlueprints/BP_FullState.BP_FullState_C")))
  ;[0.15 0.15 0.15 0.5] VFX when new state is acquired
  (Niagara|SpawnSystematLocation "/Game/VFX/NS_Transform.NS_Transform" (Math|Vector|MakeVector (.x _origin) _returnvalue (.z _origin)))
  (Niagara|SpawnSystematLocation "/Game/VFX/NS_Bang.NS_Bang" (Math|Vector|MakeVector (.x _origin) _returnvalue (.z _origin)) "0, 0, 0" "1.200000,1.200000,1.200000")
  (CallFunction|ShowNewStateAbilityUI))

(fn ShowNewStateAbilityUI
  (switch Utilities|FlowControl|Switch|SwitchonE_PlayerMoveState (Variables|Default|GetPlayerMovementState)
    (:NewEnumerator0
      (CallFunction|HideBubble :!label _label))
    (:NewEnumerator1
      (Sprite|SetFlipbook (Variables|Default|GetAnimationInstruction) "/Game/Animations/Sprites/FlipBooks/MainCharacter/FP_FrontLegJump.FP_FrontLegJump")
      (Rendering|Components|Sprite|SetSprite (Variables|Default|GetInstruction) "/Game/UI/Images/KeyboardUINew/T_Keys_Space_Sprite.T_Keys_Space_Sprite")
      (Rendering|SetVisibility (Variables|Default|GetThoughtBubble) true false :!label _label_2)
      (CallFunction|CloseAfterTime))
    (:NewEnumerator2
      (Sprite|SetFlipbook (Variables|Default|GetAnimationInstruction) "/Game/Animations/Sprites/FlipBooks/MainCharacter/FB_EarsFormGlide.FB_EarsFormGlide")
      (Rendering|Components|Sprite|SetSprite (Variables|Default|GetInstruction) "/Game/UI/Images/KeyboardUINew/T_Keys_Space_Sprite.T_Keys_Space_Sprite")
      (goto _label_2))
    (:NewEnumerator3
      (goto _label))))

(fn CloseBubblewithAction
  (params (KeyToPress :type Key%20Structure :default "None")))

(fn HideBubble
  (Rendering|SetVisibility (Variables|Default|GetThoughtBubble) false true))

(fn ShowGripStateAbilityUI
  (switch Utilities|FlowControl|Switch|SwitchonE_PlayerMoveState (Variables|Default|GetPlayerMovementState)
    (:NewEnumerator1
      (Sprite|SetFlipbook (Variables|Default|GetAnimationInstruction) "/Game/Animations/Sprites/FlipBooks/MainCharacter/FB_FrontLegGrip.FB_FrontLegGrip"))
    (:NewEnumerator2
      (Sprite|SetFlipbook (Variables|Default|GetAnimationInstruction) "/Game/Animations/Sprites/FlipBooks/MainCharacter/FB_EarsFormGripping.FB_EarsFormGripping"))
    (:NewEnumerator3
      (Sprite|SetFlipbook (Variables|Default|GetAnimationInstruction) "/Game/Animations/Sprites/FlipBooks/MainCharacter/FB_fULLGripping.FB_fULLGripping")))
  (Rendering|Components|Sprite|SetSprite (Variables|Default|GetInstruction) "/Game/UI/Images/KeyboardUINew/T_Keys_S_Sprite.T_Keys_S_Sprite")
  (Rendering|SetVisibility (Variables|Default|GetThoughtBubble) true true)
  (CallFunction|CloseAfterTime))

(fn PlayWindVFX
  (bind _thoughtbubble (Variables|Default|GetThoughtBubble))
  (Niagara|SpawnSystemAttached "/Game/VFX/NS_Wind.NS_Wind" _thoughtbubble "None" (Math|Vector|MakeVector (* (.x (.BoxExtent (Collision|GetComponentBounds _thoughtbubble))) 2.0) 0.0 0.0) "0, 0, 0" "KeepRelativeOffset" true))