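; BP_EnvironmentManager runs wind gusts that shake the camera and push the player character, skipped while the player is respawning.
; Key 1 or a debug event starts a gust: wind VFX, a sound, and the RampUpWind timeline driving strength, then audio fade-out.
; CheckPlayerLevel maps movement state to a level and shows a one-time grip prompt.
; The level-based timeline loop that would repeat gusts is unconnected and never runs.
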(event Custom|RunEnvironmentEffects
  (bind _asbp_player_character (Utilities|Casting|CastToBP_PlayerCharacter (Game|GetPlayerCharacter 0)))
  (if (not (Variables|/Game/Blueprints/BP_PlayerCharacter.BP_PlayerCharacter_C|GetIsRespawning _asbp_player_character))
    (Default|PlayWindVFX (Variables|Default|GetPlayerRef))
    (bind _returnvalue (Audio|SpawnSound2D "/Game/Audio/SoundEffects/vacuum_cleaner__1_.vacuum_cleaner__1_" 0.25 1.0 0.0 0))
    (Variables|Default|SetVacSound _returnvalue)
    (bind _scaling_wind (Timeline|RampUpWind PlayFromStart)
      (:Update
        (Game|Feedback|ClientStartCameraShake (Game|GetPlayerController 0) "/Game/Blueprints/Environment/BP_CameraShake.BP_CameraShake_C" _scaling_wind "CameraLocal" "0, 0, 0")
        (Default|BlowCharacter _asbp_player_character _scaling_wind))
      (:Finished
        (Audio|Components|Audio|FadeOut (Variables|Default|GetVacSound) 8.0 0.0 "Logarithmic" :!class /Script/Engine.AudioComponent)))))

(event Custom|DebugEnviroTrigger
  (CallFunction|RunEnvironmentEffects))

(event Custom|StopAllTimelines
  (Audio|Components|Audio|FadeOut (Variables|Default|GetVacSound) 8.0 0.0 "Logarithmic" :!class /Script/Engine.AudioComponent)
  (bind _scaling_wind (Timeline|RampUpWind Stop)
    (:Update
      (Game|Feedback|ClientStartCameraShake (Game|GetPlayerController 0) "/Game/Blueprints/Environment/BP_CameraShake.BP_CameraShake_C" _scaling_wind "CameraLocal" "0, 0, 0")
      (Default|BlowCharacter (stale Custom|RunEnvironmentEffects _asbp_player_character) _scaling_wind))
    (:Finished
      (Audio|Components|Audio|FadeOut (Variables|Default|GetVacSound) 8.0 0.0 "Logarithmic" :!class /Script/Engine.AudioComponent))))

(event EventBeginPlay
  (bind _asbp_player_character (Utilities|Casting|CastToBP_PlayerCharacter (Game|GetPlayerCharacter 0)))
  (Variables|Default|SetPlayerRef _asbp_player_character))

(event Collision|EventActorBeginOverlap
  (params (OtherActor :type Actor%20Object%20Reference)))

(event EventTick
  (params (DeltaSeconds :type Float%20%28single-precision%29)))

(event Input|KeyboardEvents|1
  (params (Key :type Key%20Structure :default "None"))
  (:Pressed
    (CallFunction|RunEnvironmentEffects)))

(fn ConstructionScript)

(fn CheckPlayerLevel
  ;[0.15 0.15 0.15 0.5] Check player level (e.g how close are they to finishing the game for environment strength)
  (bind _asbp_player_character (Utilities|Casting|CastToBP_PlayerCharacter (Game|GetPlayerCharacter 0)))
  (switch Utilities|FlowControl|Switch|SwitchonE_PlayerMoveState (Variables|/Game/Blueprints/BP_PlayerCharacter.BP_PlayerCharacter_C|GetPlayerMovementState _asbp_player_character)
    (:NewEnumerator0
      _)
    (:NewEnumerator1
      (if (Variables|Default|GetHasShownPrompt)
        _
        (else
          (Utilities|ShowFirstPrompt))))
    (:NewEnumerator2
      (if (Variables|Default|GetHasShownPrompt)
        _
        (else
          (Utilities|ShowFirstPrompt)))
      (bind _output_get (Variables|Default|SetPlayerLevel 2))
      (return _output_get))
    (:NewEnumerator3
      (if (Variables|Default|GetHasShownPrompt)
        _
        (else
          (Utilities|ShowFirstPrompt)))
      (bind _output_get_2 (Variables|Default|SetPlayerLevel 3))
      (return _output_get_2)))
  (bind _output_get_3 (Variables|Default|SetPlayerLevel 1))
  (return _output_get_3))