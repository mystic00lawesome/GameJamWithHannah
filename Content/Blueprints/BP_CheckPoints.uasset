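; Checkpoint actor that respawns the player after falling into a death box.
; Two respawn boxes record the most recently touched one as the respawn point.
; On death it freezes and hides the player, stops the environment manager's timelines and plays dust and sound effects.
; After a short delay it moves the player to that box and restores visibility, input and walking.
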(event OnComponentBeginOverlap(DeathBox)
  (params (OverlappedComponent :type Primitive%20Component%20Object%20Reference) (OtherActor :type Actor%20Object%20Reference) (OtherComp :type Primitive%20Component%20Object%20Reference) (OtherBodyIndex :type Integer) (bFromSweep :type Boolean) (SweepResult :type Hit%20Result%20Structure%20%28by%20ref%29))
  (Utilities|Casting|CastToBP_PlayerCharacter OtherActor)
  (CallFunction|RunDeath))

(event OnComponentBeginOverlap(RespawnBox1)
  (params (OverlappedComponent :type Primitive%20Component%20Object%20Reference) (OtherActor :type Actor%20Object%20Reference) (OtherComp :type Primitive%20Component%20Object%20Reference) (OtherBodyIndex :type Integer) (bFromSweep :type Boolean) (SweepResult :type Hit%20Result%20Structure%20%28by%20ref%29))
  (Utilities|Casting|CastToBP_PlayerCharacter OtherActor)
  (Variables|Default|SetMostRecentBox (Variables|Default|GetRespawnBox1)))

(event OnComponentBeginOverlap(RespawnBox2)
  (params (OverlappedComponent :type Primitive%20Component%20Object%20Reference) (OtherActor :type Actor%20Object%20Reference) (OtherComp :type Primitive%20Component%20Object%20Reference) (OtherBodyIndex :type Integer) (bFromSweep :type Boolean) (SweepResult :type Hit%20Result%20Structure%20%28by%20ref%29))
  (Utilities|Casting|CastToBP_PlayerCharacter OtherActor)
  (Variables|Default|SetMostRecentBox (Variables|Default|GetRespawnBox2)))

(event Custom|RunDeath
  (bind _playerref (Variables|Default|GetPlayerRef))
  (bind _mostrecentbox (Variables|Default|GetMostRecentBox))
  (bind _playerref_2 (Variables|Default|GetPlayerRef))
  (bind _returnvalue (Transformation|GetWorldLocation _mostrecentbox))
  (bind _charactermovement (Variables|/Script/Engine.Character|GetCharacterMovement _playerref_2))
  (Development|PrintString "Player has fallen")
  (Input|SetIgnoreMoveInput (Game|GetPlayerController 0) true)
  ;[0.15 0.15 0.15 0.5] Stop shaking
  (Variables|/Game/Blueprints/BP_PlayerCharacter.BP_PlayerCharacter_C|SetIsRespawning _playerref true)
  (bind _returnvalue_2 (Actor|GetActorOfClass "/Game/Blueprints/Environment/BP_EnvironmentManager.BP_EnvironmentManager_C"))
  (Default|StopAllTimelines _returnvalue_2)
  (Rendering|SetActorHiddenInGame _playerref_2 true)
  (Components|Movement|StopMovementImmediately _charactermovement)
  (Pawn|Components|CharacterMovement|SetMovementMode _charactermovement "MOVE_None" 0)
  (Niagara|SpawnSystematLocation "/Game/VFX/NS_DustPoof.NS_DustPoof" (Transformation|GetActorLocation _playerref_2) "0, 0, 0" "1.500000,1.500000,1.500000")
  (Audio|PlaySound2D "/Game/Audio/SoundEffects/Whimper.Whimper" 1.0 1.0 0.0 0 0)
  (Audio|PlaySound2D "/Game/Audio/SoundEffects/Respawn.Respawn" 1.0 1.0 0.0 0 0)
  (Utilities|FlowControl|Delay 3.0)
  (Audio|PlaySound2D "/Game/Audio/SoundEffects/Respawn.Respawn" 1.0 1.0 0.0 0 0 false)
  (Transformation|SetActorLocation _playerref _returnvalue false false)
  (Niagara|SpawnSystematLocation "/Game/VFX/NS_DustPoof.NS_DustPoof" _returnvalue "0, 0, 0" "1.500000,1.500000,1.500000")
  (Input|SetIgnoreMoveInput (Game|GetPlayerController 0) false)
  (Rendering|SetActorHiddenInGame _playerref false)
  (Variables|/Game/Blueprints/BP_PlayerCharacter.BP_PlayerCharacter_C|SetIsRespawning _playerref false)
  (Pawn|Components|CharacterMovement|SetMovementMode (Variables|/Script/Engine.Character|GetCharacterMovement (Variables|Default|GetPlayerRef)) "MOVE_Walking" 0))

(event EventBeginPlay
  (bind _asbp_player_character (Utilities|Casting|CastToBP_PlayerCharacter (Game|GetPlayerCharacter 0)))
  (Variables|Default|SetPlayerRef _asbp_player_character))

(event Collision|EventActorBeginOverlap
  (params (OtherActor :type Actor%20Object%20Reference)))

(event EventTick
  (params (DeltaSeconds :type Float%20%28single-precision%29)))

(fn ConstructionScript)