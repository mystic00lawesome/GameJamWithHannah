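; Parent Blueprint for collectible items wanted by NPCs, picked up when the player overlaps the item's sphere.
; On overlap it passes its class to BP_PlayerCharacter's SetCollectedItems and stops its RotatingMovement.
; It then turns to a yaw offset from the camera, scales up through the GrowQuickly timeline as pickup feedback, and destroys itself when finished.
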(event OnComponentBeginOverlap(Sphere)
  (params (OverlappedComponent :type Primitive%20Component%20Object%20Reference) (OtherActor :type Actor%20Object%20Reference) (OtherComp :type Primitive%20Component%20Object%20Reference) (OtherBodyIndex :type Integer) (bFromSweep :type Boolean) (SweepResult :type Hit%20Result%20Structure%20%28by%20ref%29))
  (bind _returnvalue (Game|GetPlayerCharacter 0))
  (if (== OtherActor _returnvalue)
    (bind _asbp_player_character (Utilities|Casting|CastToBP_PlayerCharacter _returnvalue))
    (Default|SetCollectedItems _asbp_player_character (Utilities|GetClass self))
    (Components|Activation|Deactivate (Variables|Default|GetRotatingMovement))
    (Transformation|SetActorRotation (Math|Rotator|MakeRotator 0.0 0.0 (+ (.Yaw (Math|Rotator|BreakRotator (Camera|GetCameraRotation (Game|GetPlayerCameraManager 0)))) 9e+01)))
    (bind _growitem (Timeline|GrowQuickly PlayFromStart)
      (:Update
        (Transformation|SetActorScale3D (Math|Vector|MakeVector (Math|Float|Lerp 1.0 1.9 _growitem) (Math|Float|Lerp 1.0 1.9 _growitem) (Math|Float|Lerp 1.0 1.9 _growitem))))
      (:Finished
        (Actor|DestroyActor)))))

(event EventBeginPlay)

(event Collision|EventActorBeginOverlap
  (params (OtherActor :type Actor%20Object%20Reference)))

(event EventTick
  (params (DeltaSeconds :type Float%20%28single-precision%29)))

(fn ConstructionScript)